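; BP_Crab is an environment crab that walks back and forth along world X on its own.
; Each Tick a Visibility line trace angles down and ahead along Direction, and movement input is added only if it hits, so the crab stops pushing at drops.
; A counter tracks consecutive ticks with zero X velocity and reverses Direction at its threshold, so the pause before turning depends on frame rate.
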(event `self.ReceiveTick`
  (params (DeltaSeconds :type "Float (single-precision)"))
  (bind _velocity_x (`KismetMathLibrary.BreakVector` (`MovementComponent.Velocity` (`self.CharacterMovement`))))
  (if (>= (`self.StopTime`) 30)
    (set `self.Direction` (* (`self.Direction`) -1))
    (set `self.StopTime` 0)
    (else
      (bind _newparam (`self.raytrace`))
      (if _newparam
        (`self.AddMovementInput` (`KismetMathLibrary.MakeVector` (`KismetMathLibrary.Conv_IntToDouble` (`self.Direction`)))))
      (if (== _velocity_x 0.0)
        (`/Engine/EditorBlueprintResources/StandardMacros.IncrementInt` (`self.StopTime`))
        (else
          (set `self.StopTime` 0))))))

(fn `raytrace`
  (returns (NewParam :type Boolean))
  (bind _returnvalue (`SceneComponent.K2_GetComponentLocation` (`self.Mesh`)))
  (bind (_outhit _returnvalue_2) (`KismetSystemLibrary.LineTraceSingle` _returnvalue (+ _returnvalue (* (`self.GetActorUpVector`) -50) (* (`self.Direction`) 150 (`self.GetActorForwardVector`))) "TraceTypeQuery1"))
  (return _returnvalue_2))

(fn `UserConstructionScript`)