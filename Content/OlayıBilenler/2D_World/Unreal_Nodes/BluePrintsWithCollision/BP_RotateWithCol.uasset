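; Collision-triggered node in the 2D world that switches the 3D-world character between left and right, apparently as a rotation.
; Box overlap records the overlapping actor and fires a near-instant timer; end overlap clears that state.
; The timer event uses a FlipFlop to alternately play the character's ToLeft and ToRight sequences, updating its ToLeft flag.
; ExecuteEventNode is empty and PerVariableFunction only returns zero.
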(event `self.Box.OnComponentEndOverlap`
  (params (OverlappedComponent :type "PrimitiveComponent Object Reference") (OtherActor :type "Actor Object Reference") (OtherComp :type "PrimitiveComponent Object Reference") (OtherBodyIndex :type Integer))
  (set `self.IsOverlapping` false)
  (set `self.OtherActor` null))

(event `self.Box.OnComponentBeginOverlap`
  (params (OverlappedComponent :type "PrimitiveComponent Object Reference") (OtherActor :type "Actor Object Reference") (OtherComp :type "PrimitiveComponent Object Reference") (OtherBodyIndex :type Integer) (bFromSweep :type Boolean) (SweepResult :type "HitResult Structure (by ref)"))
  (set `self.IsOverlapping` true)
  (set `self.OtherActor` OtherActor)
  (`KismetSystemLibrary.K2_SetTimerDelegate` (delegate `ExecuteNodeActionnnn`) 1e-05 false true))

(event `ExecuteNodeActionnnn`
  (`/Engine/EditorBlueprintResources/StandardMacros.FlipFlop`
    (:`A`
      (`ActorSequenceComponent.PlaySequence` (`/Game/OlayıBilenler/3D_World/Character/BP_Char/BP_3DWorldChar.ToLeft` (`self.3DWORLDCHAR`)))
      (set `/Game/OlayıBilenler/3D_World/Character/BP_Char/BP_3DWorldChar.ToLeft?` true (`self.3DWORLDCHAR`)))
    (:`B`
      (`ActorSequenceComponent.PlaySequence` (`/Game/OlayıBilenler/3D_World/Character/BP_Char/BP_3DWorldChar.ToRight` (`self.3DWORLDCHAR`)))
      (set `/Game/OlayıBilenler/3D_World/Character/BP_Char/BP_3DWorldChar.ToLeft?` false (`self.3DWORLDCHAR`)))))

(event `ExecuteEventNode`)

(fn `PerVariableFunction`
  (returns (PerVariable :type "Float (double-precision)"))
  (return 0.0))

(fn `UserConstructionScript`)