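; BP_JumpWithCol is a 2D-world node Blueprint with collision that makes the 3D-world character jump when something overlaps its box.
; Begin overlap records the overlapping actor and state, then sets a very short one-shot timer that prints a debug message and calls Jump on the 3DWORLDCHAR reference.
; End overlap clears the stored state, which the jump does not check.
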(event `self.Box.OnComponentEndOverlap`
  (params (OverlappedComponent :type "PrimitiveComponent Object Reference") (OtherActor :type "Actor Object Reference") (OtherComp :type "PrimitiveComponent Object Reference") (OtherBodyIndex :type Integer))
  (set `self.IsOverlapping` false)
  (set `self.OtherActor` null))

(event `self.Box.OnComponentBeginOverlap`
  (params (OverlappedComponent :type "PrimitiveComponent Object Reference") (OtherActor :type "Actor Object Reference") (OtherComp :type "PrimitiveComponent Object Reference") (OtherBodyIndex :type Integer) (bFromSweep :type Boolean) (SweepResult :type "HitResult Structure (by ref)"))
  (set `self.IsOverlapping` true)
  (set `self.OtherActor` OtherActor)
  (`KismetSystemLibrary.K2_SetTimerDelegate` (delegate `ExecuteNodeAcitonnn`) 0.01 false true))

(event `ExecuteNodeAcitonnn`
  (`KismetSystemLibrary.PrintString` "Jump")
  (`Character.Jump` (`self.3DWORLDCHAR`)))

(fn `PerVariableFunction`
  (returns (PerVariable :type "Float (double-precision)"))
  (return 0.0))

(fn `UserConstructionScript`)