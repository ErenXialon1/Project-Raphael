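; A 2D-world node with a collision box that makes the 3D world character jump repeatedly while it is overlapped.
; Overlaps by the 2D character, briefcase or PerFrame actors are tracked in an array, with debug prints of its count.
; A lone character or briefcase starts a looping jump timer at the Timer interval, while a PerFrame actor supplies its own interval and pauses that default timer.
; Both timers pause when the array empties.
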(event `self.Box.OnComponentEndOverlap`
  (params (OverlappedComponent :type "PrimitiveComponent Object Reference") (OtherActor :type "Actor Object Reference") (OtherComp :type "PrimitiveComponent Object Reference") (OtherBodyIndex :type Integer))
  (bind _overlappingactors (`self.OverlappingActors`))
  (bind _asbp_2dworld_character (cast `/Game/OlayıBilenler/2D_World/BP_Char/BP_2DWorldCharacter` OtherActor)
    (:`then`
      (bind _returnvalue (`KismetArrayLibrary.Array_RemoveItem` _overlappingactors _asbp_2dworld_character)))
    (:`CastFailed`
      (bind _asbp_2dbriefcase (cast `/Game/OlayıBilenler/2D_World/ControllerBox/Blueprints/BP_2DBriefcase` OtherActor)
        (:`then`
          (bind _returnvalue_2 (`KismetArrayLibrary.Array_RemoveItem` _overlappingactors _asbp_2dbriefcase)))
        (:`CastFailed`
          (bind _asper_frame (cast `/Game/OlayıBilenler/2D_World/ControllerBox/Blueprints/PerFrame` OtherActor))
          (bind _returnvalue_3 (`KismetArrayLibrary.Array_RemoveItem` _overlappingactors _asper_frame))))))
  (`KismetSystemLibrary.PrintString` (`KismetStringLibrary.Conv_IntToString` (`KismetArrayLibrary.Array_Length` _overlappingactors)))
  (if _returnvalue
    (if (not (> (`KismetArrayLibrary.Array_Length` (`self.OverlappingActors`)) 0))
      (set `self.IsOverlapping` false)
      (`self.PauseNodeAction`)
      (`self.PauseEvent1`))
    (elif _returnvalue_2
      (if (not (> (`KismetArrayLibrary.Array_Length` (`self.OverlappingActors`)) 0))
        (set `self.IsOverlapping` false)
        (`self.PauseNodeAction`)
        (`self.PauseEvent1`))
      (elif _returnvalue_3
        (if (not (> (`KismetArrayLibrary.Array_Length` (`self.OverlappingActors`)) 0))
          (set `self.IsOverlapping` false)
          (`self.PauseNodeAction`)
          (`self.PauseEvent1`))))))

(event `self.Box.OnComponentBeginOverlap`
  (params (OverlappedComponent :type "PrimitiveComponent Object Reference") (OtherActor :type "Actor Object Reference") (OtherComp :type "PrimitiveComponent Object Reference") (OtherBodyIndex :type Integer) (bFromSweep :type Boolean) (SweepResult :type "HitResult Structure (by ref)"))
  (bind _overlappingactors (`self.OverlappingActors`))
  (bind _returnvalue (`KismetStringLibrary.Conv_IntToString` (`KismetArrayLibrary.Array_Length` (`self.OverlappingActors`))))
  (bind _asbp_2dworld_character (cast `/Game/OlayıBilenler/2D_World/BP_Char/BP_2DWorldCharacter` OtherActor)
    (:`then`
      (`KismetArrayLibrary.Array_Append` _overlappingactors (`|MakeArray` _asbp_2dworld_character :!type "Actor Object Reference"))
      (`KismetSystemLibrary.PrintString` _returnvalue))
    (:`CastFailed`
      (bind _asbp_2dbriefcase (cast `/Game/OlayıBilenler/2D_World/ControllerBox/Blueprints/BP_2DBriefcase` OtherActor)
        (:`then`
          (`KismetArrayLibrary.Array_Append` _overlappingactors (`|MakeArray` _asbp_2dbriefcase :!type "Actor Object Reference"))
          (`KismetSystemLibrary.PrintString` _returnvalue))
        (:`CastFailed`
          (bind _asper_frame (cast `/Game/OlayıBilenler/2D_World/ControllerBox/Blueprints/PerFrame` OtherActor))
          (`KismetArrayLibrary.Array_Append` _overlappingactors (`|MakeArray` _asper_frame :!type "Actor Object Reference"))
          (`KismetSystemLibrary.PrintString` _returnvalue)))))
  (set `self.IsOverlapping` true)
  (for _array_element (`self.OverlappingActors`) :!label _label
    (bind _outactors (`GameplayStatics.GetAllActorsOfClass` "/Game/OlayıBilenler/2D_World/ControllerBox/Blueprints/PerFrame.PerFrame_C"))
    (for _array_element_2 _outactors
      (if (== _array_element_2 _array_element)
        (`|ExecutionSequence`
          (:`then_0`
            (break))
          (:`then_1`
            (bind _pervariable (`/Game/OlayıBilenler/2D_World/ControllerBox/Blueprints/PerFrame.PerVariableFunction` _array_element_2))
            (bind _returnvalue_2 (`KismetSystemLibrary.K2_SetTimerDelegate` (delegate `ExecuteNodeAcitonnn`) _pervariable true true)))
          (:`then_2`
            (goto _label :!via `Break`))
          (:`then_3`
            (`self.PauseEvent1`)))
        (else
          (bind _returnvalue_3 (`GameplayStatics.GetActorOfClass` "/Game/OlayıBilenler/2D_World/BP_Char/BP_2DWorldCharacter.BP_2DWorldCharacter_C"))
          (if (== _returnvalue_3 _array_element)
            (if (not (> (`KismetArrayLibrary.Array_Length` (`self.OverlappingActors`)) 1))
              (bind _returnvalue_4 (`KismetSystemLibrary.K2_SetTimerDelegate` (delegate `StartEvent1`) (`self.Timer`) true true :!label _label_2)))
            (else
              (bind _returnvalue_5 (`GameplayStatics.GetActorOfClass` "/Game/OlayıBilenler/2D_World/ControllerBox/Blueprints/BP_2DBriefcase.BP_2DBriefcase_C"))
              (if (== _array_element _returnvalue_5)
                (if (not (> (`KismetArrayLibrary.Array_Length` (`self.OverlappingActors`)) 1))
                  (goto _label_2))))))))))

(event `PauseNodeAction`
  (`KismetSystemLibrary.K2_PauseTimerHandle` (stale `self.Box.OnComponentBeginOverlap` _returnvalue_2)))

(event `ExecuteNodeAcitonnn`
  (`Character.Jump` (`self.3DWORLDCHAR`)))

(event `PauseEvent1`
  (`KismetSystemLibrary.K2_PauseTimerHandle` (stale `self.Box.OnComponentBeginOverlap` _returnvalue_4)))

(event `StartEvent1`
  (`Character.Jump` (`self.3DWORLDCHAR`)))

(fn `PerVariableFunction`
  (returns (PerVariable :type "Float (double-precision)"))
  (return 0.0))

(fn `UserConstructionScript`)