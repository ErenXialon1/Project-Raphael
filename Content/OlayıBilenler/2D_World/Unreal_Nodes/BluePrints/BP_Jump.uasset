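; BP_Jump is a node actor in the 2D world that makes the 3D world character jump repeatedly.
; Its box records the overlapping actor, which ExecuteEventNode looks for in an array to read a period from that actor's PerVariableFunction.
; That period drives a looping timer that calls Jump, and PauseNodeAction pauses it.
; The Blueprint's own PerVariableFunction is a stub returning zero.
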(event `self.Box.OnComponentEndOverlap`
  (params (OverlappedComponent :type "PrimitiveComponent Object Reference") (OtherActor :type "Actor Object Reference") (OtherComp :type "PrimitiveComponent Object Reference") (OtherBodyIndex :type Integer))
  (set `self.IsOverlapping` false)
  (set `self.OtherActor` null))

(event `self.Box.OnComponentBeginOverlap`
  (params (OverlappedComponent :type "PrimitiveComponent Object Reference") (OtherActor :type "Actor Object Reference") (OtherComp :type "PrimitiveComponent Object Reference") (OtherBodyIndex :type Integer) (bFromSweep :type Boolean) (SweepResult :type "HitResult Structure (by ref)"))
  (set `self.IsOverlapping` true)
  (set `self.OtherActor` OtherActor))

(event `ExecuteEventNode`
  (`KismetSystemLibrary.PrintString` "444")
  (for _array_element _
    (if (== _array_element (`self.OtherActor`))
      (bind _pervariable (`/Game/OlayıBilenler/2D_World/ControllerBox/Blueprints/PerFrame.PerVariableFunction` _array_element))
      (bind _returnvalue (`KismetSystemLibrary.K2_SetTimerDelegate` (delegate `ExecuteNodeAcitonnn`) _pervariable true true)))))

(event `PauseNodeAction`
  (`KismetSystemLibrary.K2_PauseTimerHandle` (stale `ExecuteEventNode` _returnvalue)))

(event `ExecuteNodeAcitonnn`
  (`KismetSystemLibrary.PrintString` "Jump")
  (`Character.Jump` (`self.3DWORLDCHAR`)))

(fn `PerVariableFunction`
  (returns (PerVariable :type "Float (double-precision)"))
  (return 0.0))

(fn `UserConstructionScript`)