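; BP_StartNode is a trigger actor that starts the move right, move left, rotate and jump node actors in the 2D world.
; When the cached 2D character overlaps its box, a DoOnce gate calls ExecuteEventNode on the first actor found of each class.
; ResetLoopAction reopens the gate and calls PauseNodeAction on those nodes.
; The construction script caches the 2D and 3D characters, though only the 2D one is used here.
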(event `self.Box.OnComponentBeginOverlap`
  (params (OverlappedComponent :type "PrimitiveComponent Object Reference") (OtherActor :type "Actor Object Reference") (OtherComp :type "PrimitiveComponent Object Reference") (OtherBodyIndex :type Integer) (bFromSweep :type Boolean) (SweepResult :type "HitResult Structure (by ref)"))
  (if (== OtherActor (`self.2DWORLDCHAR`))
    (`/Engine/EditorBlueprintResources/StandardMacros.DoOnce` false :!label _label
      (:`Completed`
        (bind _returnvalue (`GameplayStatics.GetActorOfClass` "/Game/OlayıBilenler/2D_World/Unreal_Nodes/BluePrints/BP_MoveRight.BP_MoveRight_C"))
        (`/Engine/EditorBlueprintResources/StandardMacros.IsValid` _returnvalue
          (:`Is Valid`
            (`/Game/OlayıBilenler/2D_World/Unreal_Nodes/BluePrints/BP_MoveRight.ExecuteEventNode` _returnvalue))
          (:`Is Not Valid`
            _))
        (bind _returnvalue_2 (`GameplayStatics.GetActorOfClass` "/Game/OlayıBilenler/2D_World/Unreal_Nodes/BluePrints/BP_MoveLeft.BP_MoveLeft_C"))
        (`/Engine/EditorBlueprintResources/StandardMacros.IsValid` _returnvalue_2
          (:`Is Valid`
            (`/Game/OlayıBilenler/2D_World/Unreal_Nodes/BluePrints/BP_MoveLeft.ExecuteEventNode` _returnvalue_2))
          (:`Is Not Valid`
            _))
        (bind _returnvalue_3 (`GameplayStatics.GetActorOfClass` "/Game/OlayıBilenler/2D_World/Unreal_Nodes/BluePrints/BP_Rotate.BP_Rotate_C"))
        (`/Engine/EditorBlueprintResources/StandardMacros.IsValid` _returnvalue_3
          (:`Is Valid`
            (`/Game/OlayıBilenler/2D_World/Unreal_Nodes/BluePrints/BP_Rotate.ExecuteEventNode` _returnvalue_3))
          (:`Is Not Valid`
            _))
        (bind _returnvalue_4 (`GameplayStatics.GetActorOfClass` "/Game/OlayıBilenler/2D_World/Unreal_Nodes/BluePrints/BP_Jump.BP_Jump_C"))
        (`/Engine/EditorBlueprintResources/StandardMacros.IsValid` _returnvalue_4
          (:`Is Valid`
            (`/Game/OlayıBilenler/2D_World/Unreal_Nodes/BluePrints/BP_Jump.ExecuteEventNode` _returnvalue_4)))))))

(event `ResetLoopAction`
  (`|ExecutionSequence`
    (:`then_0`
      (goto _label :!via `Reset`))
    (:`then_1`
      (bind _returnvalue (`GameplayStatics.GetActorOfClass` "/Game/OlayıBilenler/2D_World/Unreal_Nodes/BluePrints/BP_MoveRight.BP_MoveRight_C"))
      (`/Engine/EditorBlueprintResources/StandardMacros.IsValid` _returnvalue
        (:`Is Valid`
          (`/Game/OlayıBilenler/2D_World/Unreal_Nodes/BluePrints/BP_MoveRight.PauseNodeAction` _returnvalue))
        (:`Is Not Valid`
          _))
      (bind _returnvalue_2 (`GameplayStatics.GetActorOfClass` "/Game/OlayıBilenler/2D_World/Unreal_Nodes/BluePrints/BP_MoveLeft.BP_MoveLeft_C"))
      (`/Engine/EditorBlueprintResources/StandardMacros.IsValid` _returnvalue_2
        (:`Is Valid`
          (`/Game/OlayıBilenler/2D_World/Unreal_Nodes/BluePrints/BP_MoveLeft.PauseNodeAction` _returnvalue_2))
        (:`Is Not Valid`
          _))
      (bind _returnvalue_3 (`GameplayStatics.GetActorOfClass` "/Game/OlayıBilenler/2D_World/Unreal_Nodes/BluePrints/BP_Rotate.BP_Rotate_C"))
      (`/Engine/EditorBlueprintResources/StandardMacros.IsValid` _returnvalue_3
        (:`Is Valid`
          (`/Game/OlayıBilenler/2D_World/Unreal_Nodes/BluePrints/BP_Rotate.PauseNodeAction` _returnvalue_3))
        (:`Is Not Valid`
          _))
      (bind _returnvalue_4 (`GameplayStatics.GetActorOfClass` "/Game/OlayıBilenler/2D_World/Unreal_Nodes/BluePrints/BP_Jump.BP_Jump_C"))
      (`/Engine/EditorBlueprintResources/StandardMacros.IsValid` _returnvalue_4
        (:`Is Valid`
          (`/Game/OlayıBilenler/2D_World/Unreal_Nodes/BluePrints/BP_Jump.PauseNodeAction` _returnvalue_4))))))

(fn `UserConstructionScript`
  (bind _returnvalue (`GameplayStatics.GetActorOfClass` "/Game/OlayıBilenler/2D_World/BP_Char/BP_2DWorldCharacter.BP_2DWorldCharacter_C"))
  (set `self.2DWORLDCHAR` _returnvalue)
  (bind _returnvalue_2 (`GameplayStatics.GetActorOfClass` "/Game/OlayıBilenler/3D_World/Character/BP_Char/BP_3DWorldChar.BP_3DWorldChar_C"))
  (set `self.3DWORLDCHAR` _returnvalue_2))