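; BP_Rotate is a node actor in the 2D world that drives left/right turns of the 3D world character.
; Its Box overlap tracks the touching actor; on execute, a matching PerFrame actor's PerVariableFunction supplies the interval for a looping timer.
; Each tick flip-flops between the character's ToLeft and ToRight sequences and updates its ToLeft flag.
; PauseNodeAction pauses that timer.
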(event `self.Box.OnComponentEndOverlap`
  (params (OverlappedComponent :type "PrimitiveComponent Object Reference") (OtherActor :type "Actor Object Reference") (OtherComp :type "PrimitiveComponent Object Reference") (OtherBodyIndex :type Integer))
  (set `self.IsOverlapping` false)
  (set `self.OtherActor` null))

(event `self.Box.OnComponentBeginOverlap`
  (params (OverlappedComponent :type "PrimitiveComponent Object Reference") (OtherActor :type "Actor Object Reference") (OtherComp :type "PrimitiveComponent Object Reference") (OtherBodyIndex :type Integer) (bFromSweep :type Boolean) (SweepResult :type "HitResult Structure (by ref)"))
  (set `self.IsOverlapping` true)
  (set `self.OtherActor` OtherActor))

(event `PauseNodeAction`
  (`KismetSystemLibrary.K2_PauseTimerHandle` (stale `ExecuteEventNode` _returnvalue)))

(event `ExecuteEventNode`
  (bind _outactors (`GameplayStatics.GetAllActorsOfClass` "/Game/OlayıBilenler/2D_World/ControllerBox/Blueprints/PerFrame.PerFrame_C"))
  (for _array_element _outactors
    (if (== _array_element (`self.OtherActor`))
      (bind _pervariable (`/Game/OlayıBilenler/2D_World/ControllerBox/Blueprints/PerFrame.PerVariableFunction` _array_element))
      (bind _returnvalue (`KismetSystemLibrary.K2_SetTimerDelegate` (delegate `ExecuteNodeActionnnn`) _pervariable true true)))))

(event `ExecuteNodeActionnnn`
  (`/Engine/EditorBlueprintResources/StandardMacros.FlipFlop`
    (:`A`
      (`ActorSequenceComponent.PlaySequence` (`/Game/OlayıBilenler/3D_World/Character/BP_Char/BP_3DWorldChar.ToLeft` (`self.3DWORLDCHAR`)))
      (set `/Game/OlayıBilenler/3D_World/Character/BP_Char/BP_3DWorldChar.ToLeft?` true (`self.3DWORLDCHAR`)))
    (:`B`
      (`ActorSequenceComponent.PlaySequence` (`/Game/OlayıBilenler/3D_World/Character/BP_Char/BP_3DWorldChar.ToRight` (`self.3DWORLDCHAR`)))
      (set `/Game/OlayıBilenler/3D_World/Character/BP_Char/BP_3DWorldChar.ToLeft?` false (`self.3DWORLDCHAR`)))))

(fn `PerVariableFunction`
  (returns (PerVariable :type "Float (double-precision)"))
  (return 0.0))

(fn `UserConstructionScript`)