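; BP_2DBriefcase is a briefcase for the 2D world that can be carried or dropped.
; SetAsCarried sets the IsCarried flag, hides the paper sprite and disables collision on both the sprite and its box.
; SetAsDropped clears the flag, shows the sprite again and restores query-and-physics collision on the sprite and query-only on the box.
; It has no pickup logic or active Tick; both state changes come through these events.
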(event `SetAsDropped`
  ;[1 0.05857 0.4487] Dropping
  (set `self.IsCarried` false)
  (`SceneComponent.SetVisibility` (`self.PaperSprite`) true false)
  (`PrimitiveComponent.SetCollisionEnabled` (`self.PaperSprite`) "QueryAndPhysics")
  (`PrimitiveComponent.SetCollisionEnabled` (`self.Box`) "QueryOnly"))

(event `SetAsCarried`
  ;[0 0.09229 1] Carrying
  (set `self.IsCarried` true)
  (`SceneComponent.SetVisibility` (`self.PaperSprite`) false false)
  (`PrimitiveComponent.SetCollisionEnabled` (`self.PaperSprite`) "NoCollision")
  (`PrimitiveComponent.SetCollisionEnabled` (`self.Box`) "NoCollision"))

(fn `UserConstructionScript`)