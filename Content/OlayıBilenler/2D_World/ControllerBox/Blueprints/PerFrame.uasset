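; PerFrame is a carriable sprite actor for the 2D world's ControllerBox, finding the world character as its carrier at BeginPlay.
; Carrying disables collision, then either hides the sprite on a briefcase class check or snaps to the carrier's carriable sprite and attaches.
; Dropping restores visibility and collision and calls detach on the carrier, with debug prints throughout.
; PerVariableFunction returns a Frequency value but is never called in this graph.
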(event `self.ReceiveBeginPlay`
  (bind _returnvalue (`GameplayStatics.GetActorOfClass` "/Game/OlayıBilenler/2D_World/BP_Char/BP_2DWorldCharacter.BP_2DWorldCharacter_C"))
  (set `self.Carrier` _returnvalue))

(event `SetAsDropped`
  ;[1 0.05857 0.4487] Dropping
  (set `self.IsCarried` false)
  (`SceneComponent.SetVisibility` (`self.PaperSprite`) true false)
  (`KismetSystemLibrary.PrintString` "per frame visible now")
  (`PrimitiveComponent.SetCollisionEnabled` (`self.PaperSprite`) "QueryAndPhysics")
  (`PrimitiveComponent.SetCollisionEnabled` (`self.Box`) "QueryOnly")
  (`KismetSystemLibrary.PrintString` "per frame colision on")
  (`self.K2_DetachFromActor` (`self.Carrier`) "KeepRelative" "KeepRelative" "KeepRelative"))

(event `SetAsCarried`
  (bind _papersprite (`self.PaperSprite`))
  ;[0 0.09229 1] Carrying
  (set `self.IsCarried` true)
  (`KismetSystemLibrary.PrintString` "perframe invisible")
  (`PrimitiveComponent.SetCollisionEnabled` _papersprite "NoCollision")
  (`PrimitiveComponent.SetCollisionEnabled` (`self.Box`) "NoCollision")
  (`KismetSystemLibrary.PrintString` "perframe no collision")
  (if (== (`GameplayStatics.GetObjectClass` _papersprite) "/Game/OlayıBilenler/2D_World/ControllerBox/Blueprints/BPC_Briefcase.BPC_Briefcase_C")
    (`SceneComponent.SetVisibility` _papersprite false false)
    (else
      (`self.K2_SetActorLocation` (`SceneComponent.K2_GetComponentLocation` (`/Game/OlayıBilenler/2D_World/BP_Char/BP_2DWorldCharacter.CarriableSprite` (`self.Carrier`))) true)
      (`self.K2_AttachToActor` (`self.Carrier`) "None" "KeepRelative" "KeepRelative" "KeepRelative"))))

(fn `PerVariableFunction`
  (returns (PerVariable :type "Float (double-precision)"))
  (return (`self.Frequency`)))

(fn `UserConstructionScript`)