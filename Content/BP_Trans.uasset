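; BP_Trans is a one-shot trigger that hands player control from the 3D character to its 2D counterpart on overlap.
; The first SwitchingPlayerController found possesses the 2D character referenced by the 3D one, while a newly created local player takes over possession of the 3D character.
; It then adds the WBP_Camera widget to the first player's viewport and flags the 3D character as not movable.
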(event `self.ReceiveActorBeginOverlap`
  (params (OtherActor :type "Actor Object Reference"))
  (if (== OtherActor (`self.3DCharacter`))
    (`/Engine/EditorBlueprintResources/StandardMacros.DoOnce` false
      (:`Completed`
        (bind _outactors (`GameplayStatics.GetAllActorsOfClass` "/Game/OlayıBilenler/Systems/SwitchingPlayerController.SwitchingPlayerController_C"))
        (`Controller.Possess` (`|GetArrayItem` _outactors) (`/Game/OlayıBilenler/3D_World/Character/BP_Char/BP_3DWorldChar.2DCharRef` (`self.3DCharacter`)))
        (bind _returnvalue (`GameplayStatics.CreatePlayer` 1))
        (`Controller.Possess` _returnvalue (`self.3DCharacter`))
        (bind _returnvalue_2 (`|CreateWidget` "/Game/OlayıBilenler/UI_World/Blueprints/WBP_Camera.WBP_Camera_C" (`GameplayStatics.GetPlayerController` 0)))
        (`UserWidget.AddToViewport` _returnvalue_2 0)
        (set `/Game/OlayıBilenler/3D_World/Character/BP_Char/BP_3DWorldChar.IsMovable` false (`self.3DCharacter`))))))

(fn `UserConstructionScript`)